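; Boarded-up window for a VR scene whose boards are knocked loose with a crowbar pickup.
; Three trigger boxes each react once to the crowbar, dropping the next board still attached by enabling physics, ignoring Pawn collision, decrementing a counter and playing a sound.
; A separate box toggles player input and a gate for the motion controller pawn; the gate is entered when no boards remain, but shows no follow-on action.
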(event `self.Box0.OnComponentBeginOverlap`
  (params (OverlappedComponent :type "PrimitiveComponent Object Reference") (OtherActor :type "Actor Object Reference") (OtherComp :type "PrimitiveComponent Object Reference") (OtherBodyIndex :type Integer) (bFromSweep :type Boolean) (SweepResult :type "HitResult Structure (by ref)"))
  (cast `/Game/VirtualRealityBP/Blueprints/BP_PickupCrowbar` OtherActor)
  (`/Engine/EditorBlueprintResources/StandardMacros.DoOnce` false
    (:`Completed`
      ;[1 1 1] Enable Board Break
      (if (== (`self.Boards`) 0) :!label _label
        (`/Engine/EditorBlueprintResources/StandardMacros.Gate` true :!label _label_2)
        (else
          (`self.Remove Boards`))))))

(event `self.Box1.OnComponentBeginOverlap`
  (params (OverlappedComponent :type "PrimitiveComponent Object Reference") (OtherActor :type "Actor Object Reference") (OtherComp :type "PrimitiveComponent Object Reference") (OtherBodyIndex :type Integer) (bFromSweep :type Boolean) (SweepResult :type "HitResult Structure (by ref)"))
  (cast `/Game/VirtualRealityBP/Blueprints/BP_PickupCrowbar` OtherActor)
  (`/Engine/EditorBlueprintResources/StandardMacros.DoOnce` false
    (:`Completed`
      (goto _label))))

(event `self.Box2.OnComponentBeginOverlap`
  (params (OverlappedComponent :type "PrimitiveComponent Object Reference") (OtherActor :type "Actor Object Reference") (OtherComp :type "PrimitiveComponent Object Reference") (OtherBodyIndex :type Integer) (bFromSweep :type Boolean) (SweepResult :type "HitResult Structure (by ref)"))
  (cast `/Game/VirtualRealityBP/Blueprints/BP_PickupCrowbar` OtherActor)
  (`/Engine/EditorBlueprintResources/StandardMacros.DoOnce` false
    (:`Completed`
      (goto _label))))

(event `self.Box.OnComponentBeginOverlap`
  (params (OverlappedComponent :type "PrimitiveComponent Object Reference") (OtherActor :type "Actor Object Reference") (OtherComp :type "PrimitiveComponent Object Reference") (OtherBodyIndex :type Integer) (bFromSweep :type Boolean) (SweepResult :type "HitResult Structure (by ref)"))
  ;[1 1 1] Enable Board Break
  (cast `/Game/VirtualRealityBP/Blueprints/MotionControllerPawn` OtherActor)
  (`self.EnableInput` (`GameplayStatics.GetPlayerController` 0))
  (goto _label_2 :!via `Open`))

(event `self.Box.OnComponentEndOverlap`
  (params (OverlappedComponent :type "PrimitiveComponent Object Reference") (OtherActor :type "Actor Object Reference") (OtherComp :type "PrimitiveComponent Object Reference") (OtherBodyIndex :type Integer))
  ;[1 1 1] Enable Board Break
  (cast `/Game/VirtualRealityBP/Blueprints/MotionControllerPawn` OtherActor)
  (`self.DisableInput` (`GameplayStatics.GetPlayerController` 0))
  (goto _label_2 :!via `Close`))

(event `Remove Boards`
  (bind _board1 (`self.Board1`))
  (bind _board2 (`self.Board2`))
  (bind _board0 (`self.Board0`))
  ;[1 1 1] Remove Boards
  (if (not (`SceneComponent.IsSimulatingPhysics` _board0 "None"))
    (`PrimitiveComponent.SetSimulatePhysics` _board0 true)
    (`PrimitiveComponent.SetCollisionResponseToChannel` _board0 "ECC_Pawn" "ECR_Ignore")
    (bind _result (`/Engine/EditorBlueprintResources/StandardMacros.DecrementInt` (`self.Boards`) :!label _label_3)
      (:`  `
        (set `self.Boards` _result)
        ;[1 1 1] Sound Effect
        (`GameplayStatics.PlaySoundAtLocation` "/Game/RubensSoundDesignStuff/Iteration4/BoardsFalling.BoardsFalling" (`self.K2_GetActorLocation`) (struct) 1.0 1.0 0.0 null null null)))
    (elif (not (`SceneComponent.IsSimulatingPhysics` _board1 "None"))
      (`PrimitiveComponent.SetSimulatePhysics` _board1 true)
      (`PrimitiveComponent.SetCollisionResponseToChannel` _board1 "ECC_Pawn" "ECR_Ignore")
      (goto _label_3)
      (elif (not (`SceneComponent.IsSimulatingPhysics` _board2 "None"))
        (`PrimitiveComponent.SetSimulatePhysics` _board2 true)
        (`PrimitiveComponent.SetCollisionResponseToChannel` _board2 "ECC_Pawn" "ECR_Ignore")
        (goto _label_3)))))

(fn `UserConstructionScript`)