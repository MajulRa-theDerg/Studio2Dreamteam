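; BP_HoverComponent is a scene component that hovers its owner above surfaces using physics forces.
; Each tick it line-traces on the Visibility channel straight down in world space over the Height distance.
; On a hit, it pushes the owner's primitive component at its own location along the impact normal, transformed by the component's transform.
; The force fades linearly from Strength to zero as hit distance approaches Height.
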(event `self.ReceiveBeginPlay`)

(event `self.ReceiveTick`
  (params (DeltaSeconds :type "Float (single-precision)"))
  (bind _returnvalue (`self.K2_GetComponentLocation`))
  ;[1 1 1] Line Trace for HoverComp
  (bind (_outhit _returnvalue_2) (`KismetSystemLibrary.LineTraceSingle` _returnvalue (- _returnvalue (* (`KismetMathLibrary.GetUpVector` (struct)) (`self.Height`))) "TraceTypeQuery1"))
  (if _returnvalue_2
    (bind (_bblockinghit _binitialoverlap _time _distance _location _impactpoint _normal _impactnormal) (`GameplayStatics.BreakHitResult` _outhit))
    (`PrimitiveComponent.AddForceAtLocation` (`Actor.GetComponentByClass` (`self.GetOwner`) "/Script/Engine.PrimitiveComponent") (* (`KismetMathLibrary.TransformDirection` (`self.K2_GetComponentToWorld`) _impactnormal) (`KismetMathLibrary.Lerp` (`self.Strength`) 0.0 (/ _distance (`self.Height`)))) (`self.K2_GetComponentLocation`) "None")))