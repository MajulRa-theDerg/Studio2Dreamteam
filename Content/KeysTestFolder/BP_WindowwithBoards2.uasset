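; VR boarded-up window Blueprint that is broken open by hitting it with a crowbar pickup.
; Three one-shot overlap boxes each trigger RemoveBoards, which drops the next board via physics, ignores Pawn collision, counts it and plays a sound.
; Hits attempt controller rumble through the owner cast; the third also calls the vampire window event and prints a win.
; A separate volume toggles input while the motion controller pawn is inside.
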(event `self.Box0.OnComponentBeginOverlap`
  (params (OverlappedComponent :type "PrimitiveComponent Object Reference") (OtherActor :type "Actor Object Reference") (OtherComp :type "PrimitiveComponent Object Reference") (OtherBodyIndex :type Integer) (bFromSweep :type Boolean) (SweepResult :type "HitResult Structure (by ref)"))
  ;[1 1 1] Crowbar Hit Board
  (cast `/Game/VirtualRealityBP/Blueprints/BP_PickupCrowbar` OtherActor)
  (`/Engine/EditorBlueprintResources/StandardMacros.DoOnce` false
    (:`Completed`
      ;[1 1 1] Enable Board Break
      (if (== (`self.Boards2`) 2) :!label _label
        (`self.Remove Boards`)
        ;[1 1 1] Trigger Volumes for Light DMG
        (`/Game/VirtualRealityBP/Blueprints/BP_MotionController.RumbleController` (stale _asbp_motion_controller) 0.0)
        (`KismetSystemLibrary.Delay` 1.0)
        (`self.VampireWindow`)
        (`KismetSystemLibrary.PrintString` "WIN")
        (else
          ;[1 1 1] Rumble
          (`self.Remove Boards`)
          (bind _asbp_motion_controller (cast `/Game/VirtualRealityBP/Blueprints/BP_MotionController` (`self.GetOwner`)))
          (`/Game/VirtualRealityBP/Blueprints/BP_MotionController.RumbleController` _asbp_motion_controller 0.0))))))

(event `self.Box1.OnComponentBeginOverlap`
  (params (OverlappedComponent :type "PrimitiveComponent Object Reference") (OtherActor :type "Actor Object Reference") (OtherComp :type "PrimitiveComponent Object Reference") (OtherBodyIndex :type Integer) (bFromSweep :type Boolean) (SweepResult :type "HitResult Structure (by ref)"))
  ;[1 1 1] Crowbar Hit Board
  (cast `/Game/VirtualRealityBP/Blueprints/BP_PickupCrowbar` OtherActor)
  (`/Engine/EditorBlueprintResources/StandardMacros.DoOnce` false
    (:`Completed`
      (goto _label))))

(event `self.Box2.OnComponentBeginOverlap`
  (params (OverlappedComponent :type "PrimitiveComponent Object Reference") (OtherActor :type "Actor Object Reference") (OtherComp :type "PrimitiveComponent Object Reference") (OtherBodyIndex :type Integer) (bFromSweep :type Boolean) (SweepResult :type "HitResult Structure (by ref)"))
  ;[1 1 1] Crowbar Hit Board
  (cast `/Game/VirtualRealityBP/Blueprints/BP_PickupCrowbar` OtherActor)
  (`/Engine/EditorBlueprintResources/StandardMacros.DoOnce` false
    (:`Completed`
      (goto _label))))

(event `self.Box.OnComponentBeginOverlap`
  (params (OverlappedComponent :type "PrimitiveComponent Object Reference") (OtherActor :type "Actor Object Reference") (OtherComp :type "PrimitiveComponent Object Reference") (OtherBodyIndex :type Integer) (bFromSweep :type Boolean) (SweepResult :type "HitResult Structure (by ref)"))
  ;[1 1 1] Enable Board Break
  (cast `/Game/VirtualRealityBP/Blueprints/MotionControllerPawn` OtherActor)
  (`self.EnableInput` (`GameplayStatics.GetPlayerController` 0)))

(event `self.Box.OnComponentEndOverlap`
  (params (OverlappedComponent :type "PrimitiveComponent Object Reference") (OtherActor :type "Actor Object Reference") (OtherComp :type "PrimitiveComponent Object Reference") (OtherBodyIndex :type Integer))
  ;[1 1 1] Enable Board Break
  (cast `/Game/VirtualRealityBP/Blueprints/MotionControllerPawn` OtherActor)
  (`self.DisableInput` (`GameplayStatics.GetPlayerController` 0)))

(event `Remove Boards`
  (bind _board1 (`self.Board1`))
  (bind _board2 (`self.Board2`))
  (bind _board0 (`self.Board0`))
  (bind _boards2 (`self.Boards2`))
  ;[1 1 1] Remove Boards
  (if (not (`SceneComponent.IsSimulatingPhysics` _board0 "None"))
    (`PrimitiveComponent.SetSimulatePhysics` _board0 true)
    (`PrimitiveComponent.SetCollisionResponseToChannel` _board0 "ECC_Pawn" "ECR_Ignore")
    (set `self.Boards2` (+ _boards2 1) :!label _label_2)
    ;[1 1 1] Sound Effect
    (`KismetSystemLibrary.PrintString` (`KismetStringLibrary.Conv_IntToString` _boards2))
    (`GameplayStatics.PlaySoundAtLocation` "/Game/RubensSoundDesignStuff/Iteration4/BoardsFalling.BoardsFalling" (`self.K2_GetActorLocation`) (struct) 1.0 1.0 0.0 null null null)
    (elif (not (`SceneComponent.IsSimulatingPhysics` _board1 "None"))
      (`PrimitiveComponent.SetSimulatePhysics` _board1 true)
      (`PrimitiveComponent.SetCollisionResponseToChannel` _board1 "ECC_Pawn" "ECR_Ignore")
      (goto _label_2)
      (elif (not (`SceneComponent.IsSimulatingPhysics` _board2 "None"))
        (`PrimitiveComponent.SetSimulatePhysics` _board2 true)
        (`PrimitiveComponent.SetCollisionResponseToChannel` _board2 "ECC_Pawn" "ECR_Ignore")
        (goto _label_2)))))

(fn `UserConstructionScript`)