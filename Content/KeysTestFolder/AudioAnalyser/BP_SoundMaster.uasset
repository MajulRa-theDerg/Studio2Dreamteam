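; BP_SoundMaster is an audio visualizer test actor that plays a sound and scales a sphere from its spectrum.
; Playback percent updates are converted to seconds to sample channel 0 of a pre-analyzed, normalized Constant-Q (Audio Synesthesia NRT) asset.
; Each band value sets the same sphere's uniform scale at one-tenth size, so only the last band determines the visible result.
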(event `self.ReceiveBeginPlay`
  (`AudioComponent.SetSound` (`self.Audio`) (`self.Sound`))
  (set `self.Duration` (`SoundBase.Duration` (`self.Sound`)))
  (add `AudioComponent.OnAudioPlaybackPercent` (`self.Audio`) (delegate `PlaybackChange`))
  (`AudioComponent.Play` (`self.Audio`) 0.0))

(event `PlaybackChange`
  (params (PlayingSoundWave :type "SoundWave Object Reference") (PlaybackPercent :type "Float (double-precision)"))
  (set `self.PlayedTime` (* PlaybackPercent (`self.Duration`)))
  (for _array_element (`ConstantQNRT.GetNormalizedChannelConstantQAtTime` (`self.Constant_Ref`) (`self.PlayedTime`) 0)
    (`SceneComponent.SetWorldScale3D` (`self.Sphere`) (* (`KismetMathLibrary.Conv_DoubleToVector` _array_element) 0.1))))

(fn `UserConstructionScript`)